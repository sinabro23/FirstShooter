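; Shooter HUD that draws a dynamic, weapon-specific crosshair at the center of the screen.
; BeginPlay caches the player's ShooterCharacterBP, and DrawHUD re-fetches it whenever the reference is invalid.
; Each frame it draws five textures from the EquippedWeapon, shifted by half the crosshair size to center them.
; The four side pieces move outward by the character's CrosshairSpreadMultiplier times CrosshairSpreadMax, while the middle piece stays fixed.
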(event `self.ReceiveBeginPlay`
  ;[1 1 1] 직접 추가했음
  ;[1 1 1] ShooterCharacter BP 가져오기
  (`/Engine/EditorBlueprintResources/StandardMacros.IsValid` (`self.ShooterCharacter`)
    (:`Is Not Valid`
      (bind _asshooter_character_bp (cast `/Game/_Game/Character/ShooterCharacterBP` (`GameplayStatics.GetPlayerPawn` 0)))
      (set `self.ShooterCharacter` _asshooter_character_bp))))

(event `self.ReceiveDrawHUD`
  (params (SizeX :type Integer) (SizeY :type Integer))
  (bind (_x _y) (`KismetMathLibrary.BreakVector2D` (`self.ScreenCenter`)))
  (bind (_x_2 _y_2) (`KismetMathLibrary.BreakVector2D` (`self.CrosshairBaseCenter`)))
  (bind (_x_3 _y_3) (`KismetMathLibrary.BreakVector2D` (`self.CrosshairBaseCenter`)))
  (bind (_x_4 _y_4) (`KismetMathLibrary.BreakVector2D` (`self.CrosshairBaseCenter`)))
  (bind (_x_5 _y_5) (`KismetMathLibrary.BreakVector2D` (`self.CrosshairBaseCenter`)))
  (bind (_x_6 _y_6) (`KismetMathLibrary.BreakVector2D` (`self.CrosshairBaseCenter`)))
  (bind (_x_7 _y_7) (`KismetMathLibrary.BreakVector2D` (`self.CrosshairLocation`)))
  ;[1 1 1] 화면 정가운데와 크로스헤어 위치 설정
  (set `self.ScreenCenter` (`KismetMathLibrary.MakeVector2D` (`KismetMathLibrary.Conv_IntToDouble` (/ SizeX 2)) (`KismetMathLibrary.Conv_IntToDouble` (/ SizeY 2))))
  (set `self.CrosshairLocation` (`KismetMathLibrary.MakeVector2D` _x _y))
  ;[1 1 1] ShooterCharacterBP 레퍼런스를 확실하게 가져오기
  (`/Engine/EditorBlueprintResources/StandardMacros.IsValid` (`self.ShooterCharacter`)
    (:`Is Valid`
      _)
    (:`Is Not Valid`
      (bind _asshooter_character_bp (cast `/Game/_Game/Character/ShooterCharacterBP` (`GameplayStatics.GetPlayerPawn` 0)))
      (set `self.ShooterCharacter` _asshooter_character_bp)))
  ;[1 1 1] 크로스헤어 벌어질 정도 세팅
  (set `self.CrosshairMultiplier` (`ShooterCharacter.CrosshairSpreadMultiplier` (`self.ShooterCharacter`)))
  ;[1 1 1] 크로스헤어의 중간 기준점 설정
  (set `self.CrosshairBaseCenter` (`KismetMathLibrary.MakeVector2D` (- _x_7 (`self.CrosshairHalfWidth`)) (- _y_7 (`self.CrosshairHalfHeight`))))
  (`self.DrawTexture` (`Weapon.CrosshairBottom` (`ShooterCharacter.EquippedWeapon` (`self.ShooterCharacter`))) _x_4 (+ _y_4 (* (`self.CrosshairMultiplier`) (`self.CrosshairSpreadMax`))) 64.0 64.0 0.0 0.0 1.0 1.0)
  (`self.DrawTexture` (`Weapon.CrosshairTop` (`ShooterCharacter.EquippedWeapon` (`self.ShooterCharacter`))) _x_5 (- _y_5 (* (`self.CrosshairMultiplier`) (`self.CrosshairSpreadMax`))) 64.0 64.0 0.0 0.0 1.0 1.0)
  (`self.DrawTexture` (`Weapon.CrosshairLeft` (`ShooterCharacter.EquippedWeapon` (`self.ShooterCharacter`))) (- _x_6 (* (`self.CrosshairMultiplier`) (`self.CrosshairSpreadMax`))) _y_6 64.0 64.0 0.0 0.0 1.0 1.0)
  (`self.DrawTexture` (`Weapon.CrosshairRight` (`ShooterCharacter.EquippedWeapon` (`self.ShooterCharacter`))) (+ _x_2 (* (`self.CrosshairMultiplier`) (`self.CrosshairSpreadMax`))) _y_2 64.0 64.0 0.0 0.0 1.0 1.0)
  (`self.DrawTexture` (`Weapon.CrosshairMiddle` (`ShooterCharacter.EquippedWeapon` (`self.ShooterCharacter`))) _x_3 _y_3 64.0 64.0 0.0 0.0 1.0 1.0))

(fn `UserConstructionScript`)