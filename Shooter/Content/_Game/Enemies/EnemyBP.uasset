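; Enemy Blueprint that provides the UI feedback for an enemy: a health bar and floating hit numbers.
; On BeginPlay it links the HealthBar component's widget to itself and hides it, with show and hide events toggling its visibility.
; ShowHitNumber spawns a viewport widget at the screen-projected hit location, sets damage text and headshot flag, and passes it with the world location to StoreHitNumber.
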(event `self.ReceiveBeginPlay`
  (bind _asenemy_health_bar_bp (cast `/Game/_Game/HUD/EnemyHealthBarBP` (`WidgetComponent.GetUserWidgetObject` (`self.HealthBar`))))
  (set `/Game/_Game/HUD/EnemyHealthBarBP.Enemy` self _asenemy_health_bar_bp)
  (`Widget.SetVisibility` (`WidgetComponent.GetUserWidgetObject` (`self.HealthBar`)) "Hidden"))

(event `self.ShowHealthBar`
  (`Widget.SetVisibility` (`WidgetComponent.GetUserWidgetObject` (`self.HealthBar`)) "Visible")
  (`parent.ShowHealthBar`))

(event `self.HideHealthBar`
  (`Widget.SetVisibility` (`WidgetComponent.GetUserWidgetObject` (`self.HealthBar`)) "Hidden"))

(event `self.ShowHitNumber`
  (params (Damage :type Integer) (HitLocation :type "Vector Structure") (bHeadShot :type Boolean))
  (bind _returnvalue (`|CreateWidget` "/Game/_Game/HUD/HitNumber.HitNumber_C"))
  (`UserWidget.AddToViewport` _returnvalue 0)
  (`UserWidget.SetPositionInViewport` _returnvalue (`GameplayStatics.ProjectWorldToScreen` (`GameplayStatics.GetPlayerController` 0) HitLocation) true)
  (`self.StoreHitNumber` _returnvalue HitLocation)
  (set `/Game/_Game/HUD/HitNumber.HitText` (`KismetTextLibrary.Conv_IntToText` Damage) _returnvalue)
  (set `/Game/_Game/HUD/HitNumber.HeadShot` bHeadShot _returnvalue))

(fn `UserConstructionScript`)